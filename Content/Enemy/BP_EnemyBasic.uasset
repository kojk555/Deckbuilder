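; Basic enemy actor that takes on a random identity from the DT_Enemies data table on BeginPlay.
; The chosen row is stored, fills the health and name texts, and passes its moveset to BP_GameManager.
; Any damage lowers HPEnemy, updates the health text and destroys the actor at zero or below.
; HPEnemy is not set from the row's Health, which only feeds the initial display.
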(event Custom|OnTakeAnyDamage_Event
  (params (DamagedActor :type Actor%20Object%20Reference) (Damage :type Float%20%28single-precision%29) (DamageType :type Damage%20Type%20Object%20Reference) (InstigatedBy :type Controller%20Object%20Reference) (DamageCauser :type Actor%20Object%20Reference))
  (bind _output_get (Variables|Default|SetHPEnemy (- (Variables|Default|GetHPEnemy) Damage)))
  (Rendering|Components|TextRender|SetText (Variables|Default|GetHPText) (Utilities|Text|ToText(Float) _output_get "HalfToEven"))
  (if (<= (Variables|Default|GetHPEnemy) 0.0)
    (Actor|DestroyActor)))

(event EventBeginPlay
  (EventDispatchers|AssignOnTakeAnyDamage (delegate Custom|OnTakeAnyDamage_Event))
  (bind _outrownames (DataTable|GetDataTableRowNames "/Game/Enemy/DT_Enemies.DT_Enemies"))
  (bind _returnvalue (Utilities|GetDataTableRow "/Game/Enemy/DT_Enemies.DT_Enemies" (.OutItem (Utilities|Array|Random _outrownames)))
    (:then
      (Variables|Default|SetEnemyInfo _returnvalue)
      (Rendering|Components|TextRender|SetText (Variables|Default|GetHPText) (Utilities|Text|ToText(Float) (.Health (Utilities|Struct|BreakS_EnemyInfo _returnvalue)) "HalfToEven"))
      (Rendering|Components|TextRender|SetText (Variables|Default|GetNameText) (.Name (Utilities|Struct|BreakS_EnemyInfo _returnvalue)))
      (bind _returnvalue_2 (Actor|GetActorOfClass "/Game/BP_GameManager.BP_GameManager_C"))
      (Default|MovesetInfo _returnvalue_2 (.Moveset (Utilities|Struct|BreakS_EnemyInfo _returnvalue))))))

(fn ConstructionScript)