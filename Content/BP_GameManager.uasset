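; Game manager for a card battler that tracks player and enemy HP, player block and status effects, and resolves played card effects.
; ResolveEffect dispatches each effect to Damage, Block, Status stacking on the enemy, or drawing through HandRef.
; EnemyTakeDamage applies Strength, Weak and Vulnerable modifiers, and EndTurn routes Poison through it while decaying finite enemy statuses.
; Player damage handling is incomplete, ignoring its Damage input, and both death events are empty.
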(event Custom|ResolveEffect
  (params (CardInfo :type S%20Card%20Info%20Structure))
  (for _array_element (.Effect (Utilities|Struct|BreakS_CardInfo CardInfo))
    (CallFunction|ResolveSingle _array_element)))

(event Custom|ResolveSingle
  (params (Effects :type S%20Card%20Effects%20Structure))
  (bind (_effecttype _value) (Utilities|Struct|BreakS_CardEffects Effects))
  (switch Utilities|FlowControl|Switch|SwitchonE_Effects _effecttype
    (:NewEnumerator0
      (CallFunction|Damage _value))
    (:NewEnumerator1
      (CallFunction|Block _value))
    (:NewEnumerator2
      (for _array_element (.Status (Utilities|Struct|BreakS_CardInfo (stale Custom|ResolveEffect CardInfo)))
        (CallFunction|Status _array_element)))
    (:NewEnumerator3
      (CallFunction|Draw (Math|Float|Truncate _value)))))

(event Custom|EnemyTakeDamage
  (params (Damage :type Float%20%28double-precision%29))
  (Variables|Default|SetDamageVar Damage)
  (for _array_element (Variables|Default|GetPlayerStatus)
    (if (Utilities|Enum|Equal(Enum) (.Status (Utilities|Struct|BreakS_Status _array_element)) "NewEnumerator3")
      (Variables|Default|SetDamageVar (+ (Variables|Default|GetDamageVar) (.Value (Utilities|Struct|BreakS_Status _array_element))))
      (elif (Utilities|Enum|Equal(Enum) (.Status (Utilities|Struct|BreakS_Status _array_element)) "NewEnumerator2")
        (Variables|Default|SetDamageVar (* (Variables|Default|GetDamageVar) 0.7)))))
  (for _array_element_2 (Variables|Default|GetEnemyStaus)
    (if (Utilities|Enum|Equal(Enum) (.Status (Utilities|Struct|BreakS_Status _array_element_2)) "NewEnumerator1")
      (Variables|Default|SetDamageVar (* 1.3 (Variables|Default|GetDamageVar)))))
  (bind _output_get (Variables|Default|SetEnemyHp (- (Variables|Default|GetEnemyHp) (Variables|Default|GetDamageVar))))
  (if (<= (Variables|Default|GetEnemyHp) 0.0)
    (CallFunction|EnemyDie)
    (else
      (Development|PrintString (Utilities|String|ToString(Float) _output_get)))))

(event Custom|PlayerTakeDamage
  (params (Damage :type Float%20%28double-precision%29))
  (Variables|Default|SetPlayerBlock (- 0.0 (Variables|Default|GetPlayerBlock)))
  (if (< (Variables|Default|GetPlayerBlock) 0.0)
    (Variables|Default|SetPlayerHp (+ (Variables|Default|GetPlayerHp) (Variables|Default|GetPlayerBlock)))
    (Variables|Default|SetPlayerBlock 0.0)
    (if (<= (Variables|Default|GetPlayerHp) 0.0)
      _)))

(event Custom|EndTurn
  (bind _enemystaus (Variables|Default|GetEnemyStaus))
  (for (_array_element _array_index) _enemystaus
    (Utilities|FlowControl|Sequence
      (:then_0
        (switch Utilities|FlowControl|Switch|SwitchonE_Status (.Status (Utilities|Struct|BreakS_Status _array_element))
          (:NewEnumerator0
            (CallFunction|PoisonEndTurn (.Value (Utilities|Struct|BreakS_Status _array_element))))))
      (:then_1
        (if (not (.IsInfinite (Utilities|Struct|BreakS_Status _array_element)))
          (Utilities|Array|SetArrayElem _enemystaus _array_index (Utilities|Struct|MakeS_Status (.Status (Utilities|Struct|BreakS_Status _array_element)) (- (.Value (Utilities|Struct|BreakS_Status _array_element)) 1.0) (.IsInfinite (Utilities|Struct|BreakS_Status _array_element))))
          (if (<= (- (.Value (Utilities|Struct|BreakS_Status _array_element)) 1.0) 0.0)
            (Utilities|Array|RemoveIndex _enemystaus _array_index)))))))

(event Custom|EnemyDie)

(event Custom|PlayerDie)

(fn ConstructionScript)

(fn Damage
  (params (BaseDamage :type Float%20%28single-precision%29))
  (CallFunction|EnemyTakeDamage BaseDamage))

(fn Block
  (params (Value :type Float%20%28double-precision%29))
  (Variables|Default|SetPlayerBlock (+ (Variables|Default|GetPlayerBlock) Value)))

(fn Draw
  (params (Draw%20Ammount :type Integer))
  (for _index (range 1 Draw%20Ammount)
    (Default|DrawCard (Variables|Default|GethandRef))))

(fn PoisonEndTurn
  (params (Value :type Float%20%28double-precision%29))
  (CallFunction|Damage Value))

(fn Status
  (params (Status :type S%20Status%20Structure))
  (bind (_status _value _isinfinite) (Utilities|Struct|BreakS_Status Status))
  (bind _enemystaus (Variables|Default|GetEnemyStaus))
  (bind (_array_element _array_index) (Utilities|Array|ForEachLoopwithBreak _enemystaus :!label _label)
    (:LoopBody
      (if (Utilities|Enum|Equal(Enum) (.Status (Utilities|Struct|BreakS_Status _array_element)) _status)
        (Utilities|Array|SetArrayElem _enemystaus _array_index (Utilities|Struct|MakeS_Status _status (+ (.Value (Utilities|Struct|BreakS_Status _array_element)) _value) _isinfinite))
        (Variables|Default|SetFound true)
        (goto _label Break)
        (else
          (Variables|Default|SetFound false))))
    (:Completed
      (if (not (Variables|Default|GetFound))
        (Utilities|Array|Add _enemystaus (Utilities|Struct|MakeS_Status _status _value _isinfinite))))))